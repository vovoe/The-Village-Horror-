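; Component that runs the pause menu and saves and loads player state.
; Escape or P toggles PauseMenu_Widget, switching time dilation, cursor and input mode.
; Saving reads the selected slot from the master "Save" file, writes transform, time, level and health there, creates missing files then retries, and Save briefly raises a Saving flag.
; Load restores transform and health from that slot, plus sensitivity from the master file, without changing level.
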(event `Key|Escape`
  (params (Key :type "Key Structure"))
  ;[1 1 1] Pause Menu
  (:`Pressed`
    (if (`self.Pause?`) :!label _label
      (`GameplayStatics.SetGlobalTimeDilation` 1.0 :!label _label_2)
      (`Widget.RemoveFromParent` (`self.PauseWidget`))
      (set `self.Pause?` false)
      (bind _player (message `/Game/Bluprint/InterFace/IF_PlayerRef.PlayerRef` (`self.Player`)))
      (bind _controllerref (message `/Game/Bluprint/InterFace/IF_PlayerRef.ControllerRef` (`Pawn.GetController` _player)))
      (set `PlayerController.bShowMouseCursor` false _controllerref)
      (`WidgetBlueprintLibrary.SetInputMode_GameOnly` _controllerref)
      (else
        (bind _returnvalue (`|CreateWidget` "/Game/FullMainMenuAndSave/Widgets/PauseMenu_Widget.PauseMenu_Widget_C" null self))
        (bind _output_get (set `self.PauseWidget` _returnvalue))
        (`UserWidget.AddToViewport` _output_get 0)
        (`GameplayStatics.SetGlobalTimeDilation` 0.0)
        (set `self.Pause?` true)
        (bind _player_2 (message `/Game/Bluprint/InterFace/IF_PlayerRef.PlayerRef` (`self.Player`)))
        (bind _controllerref_2 (message `/Game/Bluprint/InterFace/IF_PlayerRef.ControllerRef` (`Pawn.GetController` _player_2)))
        (set `PlayerController.bShowMouseCursor` true _controllerref_2)
        (`WidgetBlueprintLibrary.SetInputMode_UIOnlyEx` _controllerref_2 null)))))

(event `Resume`
  (goto _label_2))

(event `Key|P`
  (params (Key :type "Key Structure"))
  ;[1 1 1] Pause Menu
  (:`Pressed`
    (goto _label)))

(event `PauseMenuSave`
  (bind _player (`self.Player`))
  (bind _returnvalue (`GameplayStatics.DoesSaveGameExist` "Save" :!label _label_3))
  (if _returnvalue
    (bind _returnvalue_2 (`GameplayStatics.LoadGameFromSlot` "Save"))
    (bind _assave_game_bp (cast `/Game/FullMainMenuAndSave/BP/SaveGame_BP` _returnvalue_2))
    (bind _returnvalue_3 (`|GetEnumeratorNameAsString` (`/Game/FullMainMenuAndSave/BP/SaveGame_BP.SaveSlotSelected` _assave_game_bp)))
    (bind _returnvalue_4 (`GameplayStatics.DoesSaveGameExist` _returnvalue_3))
    (if _returnvalue_4
      (bind _returnvalue_5 (`GameplayStatics.LoadGameFromSlot` _returnvalue_3))
      (bind _assave_slot_bp (cast `/Game/FullMainMenuAndSave/BP/SaveSlot_BP` _returnvalue_5))
      (set `/Game/FullMainMenuAndSave/BP/SaveSlot_BP.LocationOfThePlayer` (`Actor.K2_GetActorLocation` _player) _assave_slot_bp)
      (set `/Game/FullMainMenuAndSave/BP/SaveSlot_BP.RotationOfThePlayer` (`Actor.K2_GetActorRotation` _player) _assave_slot_bp)
      (set `/Game/FullMainMenuAndSave/BP/SaveSlot_BP.Time` (`KismetMathLibrary.Now`) _assave_slot_bp)
      (bind _returnvalue_6 (`GameplayStatics.GetCurrentLevelName` true))
      (set `/Game/FullMainMenuAndSave/BP/SaveSlot_BP.Level` _returnvalue_6 _assave_slot_bp)
      ;[1 0 0] Cast your player
      (bind _asbp_third_person_character (cast `/Game/FullMainMenuAndSave/BP/BP_ThirdPersonCharacter` _player))
      (set `/Game/FullMainMenuAndSave/BP/SaveSlot_BP.HealthOfThePlayer` (`/Game/FullMainMenuAndSave/BP/BP_ThirdPersonCharacter.Health` _asbp_third_person_character) _assave_slot_bp)
      (`GameplayStatics.SaveGameToSlot` _assave_slot_bp _returnvalue_3)
      (else
        (bind _returnvalue_7 (`GameplayStatics.CreateSaveGameObject` "/Game/FullMainMenuAndSave/BP/SaveSlot_BP.SaveSlot_BP_C"))
        (`GameplayStatics.SaveGameToSlot` _returnvalue_7 _returnvalue_3)
        (`self.Save`)))
    (else
      (bind _returnvalue_8 (`GameplayStatics.CreateSaveGameObject` "/Game/FullMainMenuAndSave/BP/SaveGame_BP.SaveGame_BP_C"))
      (`GameplayStatics.SaveGameToSlot` _returnvalue_8 "Save")
      (`self.Save`))))

(event `Save`
  ;[1 1 1] Save Game
  (`|ExecutionSequence`
    (:`then_0`
      (goto _label_3))
    (:`then_1`
      (set `self.Saving?` true)
      (`KismetSystemLibrary.Delay` 1.0)
      (set `self.Saving?` false))))

(event `Load`
  ;[1 1 1] Load
  (bind _returnvalue (`GameplayStatics.DoesSaveGameExist` "Save"))
  (if _returnvalue
    (bind _returnvalue_2 (`GameplayStatics.LoadGameFromSlot` "Save"))
    (bind _assave_game_bp (cast `/Game/FullMainMenuAndSave/BP/SaveGame_BP` _returnvalue_2))
    (bind _returnvalue_3 (`|GetEnumeratorNameAsString` (`/Game/FullMainMenuAndSave/BP/SaveGame_BP.SaveSlotSelected` _assave_game_bp)))
    (bind _returnvalue_4 (`GameplayStatics.DoesSaveGameExist` _returnvalue_3))
    (if _returnvalue_4
      (bind _returnvalue_5 (`GameplayStatics.LoadGameFromSlot` _returnvalue_3))
      (bind _assave_slot_bp (cast `/Game/FullMainMenuAndSave/BP/SaveSlot_BP` _returnvalue_5))
      (`Actor.K2_SetActorLocationAndRotation` (`self.Player`) (`/Game/FullMainMenuAndSave/BP/SaveSlot_BP.LocationOfThePlayer` _assave_slot_bp) (`/Game/FullMainMenuAndSave/BP/SaveSlot_BP.RotationOfThePlayer` _assave_slot_bp) false false)
      ;[1 0 0] Cast your player
      (bind _asbp_third_person_character (cast `/Game/FullMainMenuAndSave/BP/BP_ThirdPersonCharacter` (`self.Player`)))
      (set `/Game/FullMainMenuAndSave/BP/BP_ThirdPersonCharacter.Health` (`/Game/FullMainMenuAndSave/BP/SaveSlot_BP.HealthOfThePlayer` _assave_slot_bp) _asbp_third_person_character)
      (set `/Game/FullMainMenuAndSave/BP/BP_ThirdPersonCharacter.Sensibility` (`/Game/FullMainMenuAndSave/BP/SaveGame_BP.Sensibility` _assave_game_bp) _asbp_third_person_character))))