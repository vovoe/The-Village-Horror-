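; AC_ItemContainer is an actor component that stores items in slots and serves as the player's inventory container.
; AddItemToPlayer calls AddItem, which writes the item into the first slot with an ItemID of 0, or returns false when none is free.
; UpdateUI then gets the controller through a message to the owner and tells it to update that inventory slot, doing nothing when ResetSlot is true.
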(event `AddItemToPlayer`
  (params (Item :type "/Game/Bluprint/Structure/S_ItemInfo Structure"))
  (`self.AddItem` Item))

(fn `AddItem`
  (params (Item :type "/Game/Bluprint/Structure/S_ItemInfo Structure"))
  (returns (`Success?` :type Boolean))
  (locals (LocalItem :type "/Game/Bluprint/Structure/S_ItemInfo Structure") (LocalEmptyIndex :type Integer :default 0))
  (set `local.LocalItem` Item)
  (bind (_success_ _emptyindex) (`self.FindEmptySlot`))
  (if _success_
    (bind _output_get (set `local.LocalEmptyIndex` _emptyindex))
    (`KismetArrayLibrary.Array_Set` (`self.Item`) _output_get (`local.LocalItem`))
    (`self.UpdateUI` (`local.LocalEmptyIndex`) (`local.LocalItem`))
    (return true)
    (else
      (return false))))

(fn `FindEmptySlot`
  (returns (`Success?` :type Boolean) (EmptyIndex :type Integer))
  (locals (LocalEmptyIndex :type Integer) (`FoundEmptySlot?` :type Boolean))
  (for (_array_element _array_index) (`self.Item`)
    (if (== (`.ItemID_2_51E415E4491EB98371F50C97ADF68684` (break `/Game/Bluprint/Structure/S_ItemInfo` _array_element)) 0)
      (set `local.LocalEmptyIndex` _array_index)
      (set `local.FoundEmptySlot?` true)
      (break)))
  (return (`local.FoundEmptySlot?`) (`local.LocalEmptyIndex`)))

(fn `UpdateUI`
  (params (Index :type Integer) (ItemInfo :type "/Game/Bluprint/Structure/S_ItemInfo Structure") (`ResetSlot?` :type Boolean))
  (locals (LocalIndex :type Integer) (LocalItem :type "/Game/Bluprint/Structure/S_ItemInfo Structure"))
  (set `local.LocalIndex` Index)
  (set `local.LocalItem` ItemInfo)
  (if (not `ResetSlot?`)
    (bind _controllerref (message `/Game/Bluprint/InterFace/IF_PlayerRef.GetControllerFromChar` (`self.GetOwner`)))
    (`/Game/Bluprint/GeneralBP/PC_MainController.UpdateInventorySlot` _controllerref (`local.LocalIndex`) (`local.LocalItem`))))