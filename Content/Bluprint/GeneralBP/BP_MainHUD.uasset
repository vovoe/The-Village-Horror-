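; BP_MainHUD is a HUD Blueprint that draws the on-screen crosshair.
; Every DrawHUD it draws a small texture from the screen midpoint, with the CrossHair flag gating which texture is supplied.
; The Interact flag swaps the Crosshair texture for 90Degree_IES and slightly changes its size.
; MainHudRef returns the HUD itself as a reference.
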(event `self.ReceiveDrawHUD`
  (params (SizeX :type Integer) (SizeY :type Integer))
  (bind _returnvalue (`KismetMathLibrary.SelectFloat` 9.0 10.0 (`self.Interact?`)))
  (`self.DrawTexture` (select `bool` (`self.CrossHair?`) :`true` (select `bool` (`self.Interact?`) :`false` "/Game/Texture/UI/Test/Crosshair.Crosshair" :`true` "/Engine/EngineLightProfiles/90Degree_IES.90Degree_IES" :!type "Texture Object Reference")) (`KismetMathLibrary.Conv_IntToDouble` (/ SizeX 2)) (`KismetMathLibrary.Conv_IntToDouble` (/ SizeY 2)) _returnvalue _returnvalue))

(fn `MainHudRef`
  (returns (HudRef :type "/Game/Bluprint/GeneralBP/BP_MainHUD Object Reference"))
  (return self))

(fn `UserConstructionScript`)